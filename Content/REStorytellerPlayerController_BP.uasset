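; Player controller for the REStoryteller character that owns the on-screen action text and inventory UI.
; Setup caches the pawn and creates the text widget, which DisplayString feeds; a flag lets Tick rerun setup once.
; The Inventory action toggles a lazily created inventory screen, redirecting Turn input from the character to latched, one-step item selection.
; GetActiveInventoryItem returns that selection, but reports active even when the inventory is closed.
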(event `self.ReceiveBeginPlay`
  (`KismetSystemLibrary.PrintString` "Hello" :!label _label)
  (bind _asrestoryteller_character_bp (cast `/Game/ThirdPersonCPP/Blueprints/REStorytellerCharacter_BP` (`GameplayStatics.GetPlayerPawn` 0))
    (:`then`
      (set `self.RECharacter` _asrestoryteller_character_bp)
      (`KismetSystemLibrary.PrintString` "ThirdPersonCharacter Assigned in Controller"))
    (:`CastFailed`
      (`KismetSystemLibrary.PrintString` "ThirdPersonCharacterNotFound")))
  (bind _returnvalue (`|CreateWidget` "/Game/Blueprints/WB_TextDisplay.WB_TextDisplay_C" self))
  (bind _output_get (set `self.ActionTextDisplay` _returnvalue))
  (`KismetSystemLibrary.PrintString` "Created Action Text Display")
  (`UserWidget.AddToPlayerScreen` _output_get 0))

(event `InputAxis|Turn`
  (params (AxisValue :type "Float (single-precision)"))
  (bind _recharacter (`self.RECharacter`))
  (bind _inventorywidget (`self.InventoryWidget`))
  (bind _returnvalue (not (`self.InventorySelectionChangeMade`)))
  (if (`self.InventoryDisplayed`)
    ;[1 1 1] InventoryControl
    (if (< AxisValue 0.0)
      (if _returnvalue
        (`/Game/Blueprints/Inventory/WB_InventoryScreen.IncrementSelection` _inventorywidget)
        (set `self.InventorySelectionChangeMade` true :!label _label_2))
      (elif (> AxisValue 0.0)
        (if _returnvalue
          (`/Game/Blueprints/Inventory/WB_InventoryScreen.DecrementSelection` _inventorywidget)
          (goto _label_2))
        (else
          (set `self.InventorySelectionChangeMade` false))))
    (else
      ;[1 1 1] Character Movement
      (if (`KismetSystemLibrary.IsValid` _recharacter)
        (`REStorytellerCharacter.Turn` _recharacter AxisValue)))))

(event `self.ReceiveTick`
  (params (DeltaSeconds :type "Float (single-precision)"))
  (if (`self.BeginPlay`)
    (set `self.BeginPlay` false)
    (`KismetSystemLibrary.PrintString` "Begin Play:")
    (goto _label)))

(event `InputAction|Inventory`
  (params (Key :type "Key Structure"))
  (bind _inventorywidget (`self.InventoryWidget`))
  (:`Pressed`
    (`KismetSystemLibrary.PrintString` "Inventory Pressed")
    (if (not (`KismetSystemLibrary.IsValid` (`self.InventoryWidget`)))
      ;[1 1 1] Create the inventory Widget
      (bind _returnvalue (`|CreateWidget` "/Game/Blueprints/Inventory/WB_InventoryScreen.WB_InventoryScreen_C" self))
      (bind _output_get (set `self.InventoryWidget` _returnvalue))
      (`/Game/Blueprints/Inventory/WB_InventoryScreen.UpdateInventoryDisplay` _output_get (`REStorytellerCharacter.Inventory` (`self.RECharacter`))))
    (if (`self.InventoryDisplayed`)
      (`Widget.RemoveFromParent` _inventorywidget)
      (set `self.InventoryDisplayed` false)
      (`WidgetBlueprintLibrary.SetInputMode_GameOnly` self)
      (else
        (bind _returnvalue_2 (`UserWidget.AddToPlayerScreen` _inventorywidget 0))
        (set `self.InventoryDisplayed` _returnvalue_2)
        (`WidgetBlueprintLibrary.SetInputMode_GameAndUIEx` self null)))))

(fn `DisplayString`
  (params (TextToDisplay :type String) (TimeToDisplay :type "Float (double-precision)"))
  (returns (ReturnValue :type Boolean))
  (`/Game/Blueprints/WB_TextDisplay.Add String` (`self.ActionTextDisplay`) TextToDisplay TimeToDisplay)
  (return false))

(fn `GetActiveInventoryItem`
  (returns (InventoryActive :type Boolean) (`Selected Item` :type "ItemAbstract Object Reference") (SelectedIndex :type Integer))
  (if (and (`KismetSystemLibrary.IsValid` (`self.InventoryWidget`)) (`self.InventoryDisplayed`))
    (bind (_selecteditem _index) (`/Game/Blueprints/Inventory/WB_InventoryScreen.GetSelectedItem` (`self.InventoryWidget`)))
    (return true _selecteditem _index)
    (else
      (return true null 0))))

(fn `UserConstructionScript`)