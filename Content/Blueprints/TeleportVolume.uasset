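; Trigger volume that teleports a configured actor when a specified actor overlaps its box.
; The moved actor lands at an offset from the volume's location with a set rotation, a random rustling sound plays at the player, and a timer briefly blocks retriggering.
; The construction script applies box size and rotation and places an optional arrow previewing the destination and facing.
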(event `self.Box.OnComponentBeginOverlap`
  (params (OverlappedComponent :type "PrimitiveComponent Object Reference") (OtherActor :type "Actor Object Reference") (OtherComp :type "PrimitiveComponent Object Reference") (OtherBodyIndex :type Integer) (bFromSweep :type Boolean) (SweepResult :type "HitResult Structure (by ref)"))
  (bind _actortolookfor (`self.ActorToLookFor`))
  (bind _rustling (`self.Rustling`))
  (if (and (== OtherActor _actortolookfor) (`KismetSystemLibrary.IsValid` _actortolookfor) (`KismetSystemLibrary.IsValid` (`self.ActorToMove`)) (`self.CanTeleport`))
    (set `self.CanTeleport` false)
    (`self.K2_SetActorLocationAndRotation` (`self.ActorToMove`) (+ (`self.MoveTarget`) (`self.K2_GetActorLocation` self)) (`self.MoveRotation`) false false)
    (`KismetSystemLibrary.PrintString` "Teleport Successful")
    (`GameplayStatics.PlaySoundAtLocation` (`|GetArrayItem` _rustling (`KismetMathLibrary.RandomInteger` (`KismetArrayLibrary.Array_Length` _rustling))) (`self.K2_GetActorLocation` (`GameplayStatics.GetPlayerPawn` 0)) (struct) (`self.Volume`) 1.0 0.0 null null null)
    (`KismetSystemLibrary.K2_SetTimerDelegate` (delegate `SetTeleport Active`) 3.0)))

(event `SetTeleport Active`
  (set `self.CanTeleport` true))

(fn `UserConstructionScript`
  (bind _arrow (`self.Arrow`))
  (`BoxComponent.SetBoxExtent` (`self.Box`) (`self.Box Bounds`) true)
  (`SceneComponent.K2_AddRelativeRotation` (`self.Box`) (`self.Box rotation`) false false)
  (`SceneComponent.K2_AddRelativeRotation` (`self.Box`) (`self.Box rotation`) false false)
  (`SceneComponent.K2_AddRelativeLocation` _arrow (`self.MoveTarget`) false false)
  (`SceneComponent.K2_AddLocalRotation` _arrow (`self.MoveRotation`) false false)
  (`SceneComponent.SetVisibility` (`self.Arrow`) (`self.Show rotation Arrow`) false))